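; VR pawn for the main menu that sets up head-mounted tracking and lets both hands click on widgets.
; On BeginPlay it hides the mouse cursor and picks the tracking origin by headset: floor for Oculus and SteamVR, eye level plus a height offset for PSVR.
; It spawns left and right VRMenuHands attached to the VR origin.
; The left and right teleport inputs are reused to forward click press and release to each hand.
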(event `self.ReceiveBeginPlay`
  (bind _returnvalue (`SceneComponent.K2_GetComponentToWorld` (`self.VROrigin`)))
  ;[0.2344 0.8088 1] Setup VR Camera and Hands
  (set `PlayerController.bShowMouseCursor` false (`GameplayStatics.GetPlayerController` 0))
  (`|ExecutionSequence`
    (:`then_0`
      (switch `name` (`HeadMountedDisplayFunctionLibrary.GetHMDDeviceName`)
        (:`OculusHMD`
          (`HeadMountedDisplayFunctionLibrary.SetTrackingOrigin` "Floor" :!label _label) ; Windows (Oculus / Vive)
        )
        (:`SteamVR`
          (goto _label))
        (:`PSVR`
          (`HeadMountedDisplayFunctionLibrary.SetTrackingOrigin` "Eye") ; PS4
          (`SceneComponent.K2_AddLocalOffset` (`self.VROrigin`) (`KismetMathLibrary.MakeVector` 0.0 0.0 (`self.CameraHeight`)) false false))))
    (:`then_1`
      (bind _returnvalue_2 (`|SpawnActorFromClass` "/Game/MyContent/MainMenu/Blueprints/VRMenuHands.VRMenuHands_C" _returnvalue "Undefined" "OverrideRootScale" self false null))
      (set `self.RightController` _returnvalue_2)
      (`self.K2_AttachToComponent` (`self.VROrigin`) "None" "SnapToTarget" "SnapToTarget" "KeepWorld")
      (bind _returnvalue_3 (`|SpawnActorFromClass` "/Game/MyContent/MainMenu/Blueprints/VRMenuHands.VRMenuHands_C" _returnvalue "Undefined" "OverrideRootScale" self true null))
      (set `self.LeftController` _returnvalue_3)
      (`self.K2_AttachToComponent` (`self.VROrigin`) "None" "SnapToTarget" "SnapToTarget" "KeepWorld"))))

(event `InputAction|TeleportLeft`
  (params (Key :type "Key Structure"))
  (bind _leftcontroller (`self.LeftController`))
  ;[1 0.145 0] Interact with widget
  (:`Pressed`
    (`/Game/MyContent/MainMenu/Blueprints/VRMenuHands.Click` _leftcontroller true))
  (:`Released`
    (`/Game/MyContent/MainMenu/Blueprints/VRMenuHands.Click` _leftcontroller false)))

(event `InputAction|TeleportRight`
  (params (Key :type "Key Structure"))
  (bind _rightcontroller (`self.RightController`))
  ;[1 0.145 0] Interact with widget
  (:`Pressed`
    (`/Game/MyContent/MainMenu/Blueprints/VRMenuHands.Click` _rightcontroller true))
  (:`Released`
    (`/Game/MyContent/MainMenu/Blueprints/VRMenuHands.Click` _rightcontroller false)))

(fn `UserConstructionScript`)