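; VRMenuHands is a VR hand actor for the main menu that points at and clicks widgets.
; On BeginPlay, an IsLeft flag sets the motion controller's source to the left or right hand.
; Each tick draws a one-frame debug line trace along the widget interaction component's forward vector to show the pointer.
; A Click event with a Press boolean presses or releases the left mouse pointer key on that component.
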(event `self.ReceiveBeginPlay`
  (bind _motioncontroller (`self.MotionController`))
  ;[0.02316 0.6432 1] Attach Hands to controllers
  (if (`self.isLeft?`)
    (set `MotionControllerComponent.MotionSource` "Left" _motioncontroller)
    (else
      (set `MotionControllerComponent.MotionSource` "Right" _motioncontroller))))

(event `self.ReceiveTick`
  (params (DeltaSeconds :type "Float (single-precision)"))
  (bind _location (.location (`SceneComponent.K2_GetComponentToWorld` (`self.WidgetInteraction`))))
  ;[1 1 1] Visual trace for widget interaction
  (`KismetSystemLibrary.LineTraceSingle` :`Start` _location :`End` (+ _location (* (`KismetMathLibrary.GetForwardVector` (.rotation (`SceneComponent.K2_GetComponentToWorld` (`self.WidgetInteraction`)))) (`WidgetInteractionComponent.InteractionDistance` (`self.WidgetInteraction`)))) :`TraceChannel` "TraceTypeQuery2" :`DrawDebugType` "ForOneFrame"))

(event `Click`
  (params (Press :type Boolean))
  (bind _widgetinteraction (`self.WidgetInteraction`))
  ;[1 0.6456 0] Interact with Widget
  (if Press
    (`WidgetInteractionComponent.PressPointerKey` _widgetinteraction "LeftMouseButton")
    (else
      (`WidgetInteractionComponent.ReleasePointerKey` _widgetinteraction "LeftMouseButton"))))

(fn `UserConstructionScript`)