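; Networked VR player character that sets up the headset and two hands, with fist grips, snap turning and teleporting.
; On authority, BeginPlay sets the tracking origin by HMD type and spawns left and right VR_Hands actors attached to the Origin.
; Input drives the hands' fist and teleport functions, plus thumbstick yaw turns latched until sticks recenter.
; Remote instances push actor and camera transforms to the server every tick through ServerTick.
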(event `self.ReceiveBeginPlay`
  ;[1 0.1899 0] Setup VR Camera and Hands
  (`/Engine/EditorBlueprintResources/ActorMacros.Switch Has Authority`
    (:`Authority`
      (`self.ServerBegin`))))

(event `ServerBegin`
  (bind _returnvalue (`SceneComponent.K2_GetComponentToWorld` (`self.Origin`)))
  ;[1 0.1899 0] Setup VR Camera and Hands
  (`|ExecutionSequence`
    (:`then_0`
      (switch `name` (`HeadMountedDisplayFunctionLibrary.GetHMDDeviceName`)
        (:`OculusHMD`
          (`HeadMountedDisplayFunctionLibrary.SetTrackingOrigin` "Floor" :!label _label) ; Windows (Oculus / Vive)
        )
        (:`SteamVR`
          (goto _label))
        (:`PSVR`
          (`HeadMountedDisplayFunctionLibrary.SetTrackingOrigin` "Eye") ; PS4
          (`SceneComponent.K2_AddLocalOffset` (`self.Origin`) (`KismetMathLibrary.MakeVector` 0.0 0.0 (`self.CameraHeight`)) false false))))
    (:`then_1`
      (bind _returnvalue_2 (`|SpawnActorFromClass` "/Game/MyContent/Blueprints/GameMode/VR_Hands.VR_Hands_C" _returnvalue "Undefined" "OverrideRootScale" self false self))
      (bind _output_get (set `self.LeftController` _returnvalue_2))
      (`self.K2_AttachToComponent` _output_get (`self.Origin`) "None" "SnapToTarget" "SnapToTarget" "KeepWorld" true)
      (bind _returnvalue_3 (`|SpawnActorFromClass` "/Game/MyContent/Blueprints/GameMode/VR_Hands.VR_Hands_C" _returnvalue "Undefined" "OverrideRootScale" self true self))
      (bind _output_get_2 (set `self.RightController` _returnvalue_3))
      (`self.K2_AttachToComponent` _output_get_2 (`self.Origin`) "None" "SnapToTarget" "SnapToTarget" "KeepWorld" true))))

(event `self.ReceiveTick`
  (params (DeltaSeconds :type "Float (single-precision)"))
  ;[0 0.6339 1] Tick Update Client Transform on Server
  (`/Engine/EditorBlueprintResources/ActorMacros.Switch Has Authority`
    (:`Remote`
      (`self.ServerTick` (`SceneComponent.GetRelativeTransform` (`self.Camera`)) (`self.GetTransform`)))))

(event `ServerTick`
  (params (CameraTransform :type "Transform Structure (by ref)") (ActorTransform :type "Transform Structure (by ref)"))
  ;[0 0.6339 1] Tick Update Client Transform on Server
  (`self.K2_SetActorTransform` ActorTransform)
  (`SceneComponent.K2_SetRelativeTransform` (`self.Camera`) CameraTransform false false))

(event `InputAction|GrabLeft`
  (params (Key :type "Key Structure"))
  (bind _leftcontroller (`self.LeftController`))
  ;[0.7871 1 0] Hand Fist Animation
  (:`Pressed`
    (`/Game/MyContent/Blueprints/GameMode/VR_Hands.MakeFist` _leftcontroller true))
  (:`Released`
    (`/Game/MyContent/Blueprints/GameMode/VR_Hands.MakeFist` _leftcontroller false)))

(event `InputAction|GrabRight`
  (params (Key :type "Key Structure"))
  (bind _rightcontroller (`self.RightController`))
  ;[0.7871 1 0] Hand Fist Animation
  (:`Pressed`
    (`/Game/MyContent/Blueprints/GameMode/VR_Hands.MakeFist` _rightcontroller true))
  (:`Released`
    (`/Game/MyContent/Blueprints/GameMode/VR_Hands.MakeFist` _rightcontroller false)))

(event `InputAxis|MotionControllerThumbRight_X`
  (params (AxisValue :type "Float (single-precision)"))
  ;[1 1 1] Rotating Pawn
  (if (> (`KismetMathLibrary.Abs` AxisValue) 0.7)
    (if (not (`self.Turned?`))
      (`self.K2_AddActorWorldRotation` (`KismetMathLibrary.MakeRotator` 0.0 0.0 (* (`KismetMathLibrary.SignOfFloat` AxisValue) 45.0)))
      (set `self.Turned?` true))
    (elif (<= (`KismetMathLibrary.Abs` (`self.GetInputAxisValue`)) 0.7)
      (set `self.Turned?` false))))

(event `InputAxis|MotionControllerThumbLeft_X`
  (params (AxisValue :type "Float (single-precision)"))
  ;[1 1 1] Rotating Pawn
  (if (> (`KismetMathLibrary.Abs` AxisValue) 0.7)
    (if (not (`self.Turned?`))
      (`self.K2_AddActorWorldRotation` (`KismetMathLibrary.MakeRotator` 0.0 0.0 (* (`KismetMathLibrary.SignOfFloat` AxisValue) 45.0)))
      (set `self.Turned?` true))
    (elif (<= (`KismetMathLibrary.Abs` (`self.GetInputAxisValue`)) 0.7)
      (set `self.Turned?` false))))

(event `InputAction|TeleportLeft`
  (params (Key :type "Key Structure"))
  (bind _leftcontroller (`self.LeftController`))
  ;[0 0.4117 1] Teleportation
  (:`Pressed`
    (`/Game/MyContent/Blueprints/GameMode/VR_Hands.ActivateTeleport` (`self.LeftController`) true)
    (`/Game/MyContent/Blueprints/GameMode/VR_Hands.ActivateTeleport` (`self.RightController`) false))
  (:`Released`
    (`/Game/MyContent/Blueprints/GameMode/VR_Hands.ActivateTeleport` _leftcontroller false)
    (if (`/Game/MyContent/Blueprints/GameMode/VR_Hands.CanTeleport?` _leftcontroller)
      (bind _point (`/Game/MyContent/Blueprints/GameMode/VR_Hands.RecieveTeleportPoint` _leftcontroller))
      (`self.K2_SetActorLocation` _point))))

(event `InputAction|TeleportRight`
  (params (Key :type "Key Structure"))
  (bind _rightcontroller (`self.RightController`))
  ;[0 0.4117 1] Teleportation
  (:`Pressed`
    (`/Game/MyContent/Blueprints/GameMode/VR_Hands.ActivateTeleport` (`self.LeftController`) false)
    (`/Game/MyContent/Blueprints/GameMode/VR_Hands.ActivateTeleport` (`self.RightController`) true))
  (:`Released`
    (`/Game/MyContent/Blueprints/GameMode/VR_Hands.ActivateTeleport` _rightcontroller false)
    (if (`/Game/MyContent/Blueprints/GameMode/VR_Hands.CanTeleport?` _rightcontroller)
      (bind _point (`/Game/MyContent/Blueprints/GameMode/VR_Hands.RecieveTeleportPoint` _rightcontroller))
      (`self.K2_SetActorLocation` _point))))

(fn `UserConstructionScript`)