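; Player controller that spawns and possesses a pawn for its player, with a mouse-driven punch for PC testing.
; SpawnActor checks for an enabled headset and passes the result to ServerSpawn, which possesses a new VRCharacter or, without a headset, a SpectatorPawn.
; Left click traces under the cursor and, on a physics-simulating component, calls ServerPunch to apply an impulse along the camera-to-hit direction.
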(event `Key|LeftMouseButton`
  (params (Key :type "Key Structure"))
  (bind (_bblockinghit _binitialoverlap _time _distance _location _impactpoint _normal _impactnormal _physmat _hitactor _hitcomponent) (`GameplayStatics.BreakHitResult` (`self.GetHitResultUnderCursorByChannel` "TraceTypeQuery1")))
  ;[0.007734 0.5562 1] PC Punch testing
  (:`Pressed`
    (if _bblockinghit
      (if (`SceneComponent.IsSimulatingPhysics` _hitcomponent "None")
        (`self.ServerPunch` _hitcomponent (* (`KismetMathLibrary.GetDirectionUnitVector` (`PlayerCameraManager.GetCameraLocation` (`self.PlayerCameraManager`)) _location) 2500.0) _location)))))

(event `ServerPunch`
  (params (Target :type "PrimitiveComponent Object Reference") (Impulse :type "Vector Structure") (Location :type "Vector Structure"))
  ;[0.007734 0.5562 1] PC Punch testing
  (`/Engine/EditorBlueprintResources/StandardMacros.IsValid` Target
    (:`Is Valid`
      (`PrimitiveComponent.AddImpulseAtLocation` Target Impulse Location "None"))))

(event `Spawn Actor`
  (params (SpawnTransform :type "Transform Structure"))
  ;[1 0.3008 0.2809] Spawn Pawn on Server and check if using VR Headset
  (`self.ServerSpawn` self SpawnTransform (`HeadMountedDisplayFunctionLibrary.IsHeadMountedDisplayEnabled`)))

(event `ServerSpawn`
  (params (Target :type "PlayerController Object Reference") (SpawnTransform :type "Transform Structure") (Index :type Boolean))
  ;[1 0.3008 0.2809] Spawn Pawn on Server and check if using VR Headset
  (bind _returnvalue (`|SpawnActorFromClass` (select `bool` Index :`false` "/Script/Engine.SpectatorPawn" :`true` "/Game/MyContent/Blueprints/GameMode/VRCharacter.VRCharacter_C" :!type "Actor Class Reference") SpawnTransform "Undefined" "OverrideRootScale" Target null))
  (bind _aspawn (cast `Pawn` _returnvalue))
  (`self.Possess` Target _aspawn)
  (`self.EnableInput` _aspawn Target))

(fn `UserConstructionScript`)