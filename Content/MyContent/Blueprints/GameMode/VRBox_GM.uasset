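; VRBox_GM is a game mode that spawns each joining player at a different Player Start.
; On PostLogin it fills a map of Player Starts to controllers if empty, then claims the first start without a valid controller for the new player.
; It then casts that player to VRBox_PC and calls its SpawnActor with the start's transform, leaving the spawning to the controller.
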(event `self.K2_PostLogin`
  (params (NewPlayer :type "PlayerController Object Reference"))
  (bind _startpoints (`self.StartPoints`))
  ;[0 0 0] Get Player Start Locations and Spawn Players on different ones
  (if (not (> (`BlueprintMapLibrary.Map_Length` (`self.StartPoints`)) 0))
    ;;[1 0.6018 0] Recieve all Start Locations
    (bind _outactors (`GameplayStatics.GetAllActorsOfClass` "/Script/Engine.PlayerStart"))
    (for _array_element _outactors
      (`BlueprintMapLibrary.Map_Add` (`self.StartPoints`) _array_element)))
  (bind _keys (`BlueprintMapLibrary.Map_Keys` (`self.StartPoints`)))
  (for _array_element_2 _keys
    (`/Engine/EditorBlueprintResources/StandardMacros.IsValid` (`BlueprintMapLibrary.Map_Find` _startpoints _array_element_2)
      (:`Is Not Valid`
        (`BlueprintMapLibrary.Map_Add` _startpoints _array_element_2 NewPlayer)
        (bind _asvrbox_pc (cast `/Game/MyContent/Blueprints/GameMode/VRBox_PC` NewPlayer))
        (`/Game/MyContent/Blueprints/GameMode/VRBox_PC.Spawn Actor` _asvrbox_pc (`self.GetTransform` _array_element_2))
        (break)))))

(fn `UserConstructionScript`)