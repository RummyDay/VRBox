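; Networked VR hand actor that binds its motion controller to the left or right side, mirroring the mesh for the left.
; Fist state drives the hand's anim instance and passes through server and multicast events.
; While teleport is active, Tick traces forward, validates the hit against the navmesh and draws a color-coded debug line.
; Remote clients send the hand transform to the server every tick, and RecieveTeleportPoint returns the aimed location.
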(event `self.ReceiveBeginPlay`
  ;[0.0643 0.2771 1] Attach Hands to controllers
  (if (`self.isRightHand`)
    (set `MotionControllerComponent.MotionSource` "Right" (`self.MotionController`))
    (else
      (set `MotionControllerComponent.MotionSource` "Left" (`self.MotionController`))
      (`SceneComponent.SetRelativeScale3D` (`self.HandMesh`) (1.0 1.0 -1.0)))))

(event `MakeFist`
  (params (State :type Boolean))
  ;[0.191 0.5347 1] Update Hands State
  (message `/Game/MyContent/Blueprints/Interfaces/AnimationInterface.SendBool1` (`SkeletalMeshComponent.GetAnimInstance` (`self.HandMesh`)) State)
  (`self.ServerFist` State))

(event `ServerFist`
  (params (State :type Boolean))
  ;[0.191 0.5347 1] Update Hands State
  ;;[1 0.7169 0.121] Client update hands' state on server
  (message `/Game/MyContent/Blueprints/Interfaces/AnimationInterface.SendBool1` (`SkeletalMeshComponent.GetAnimInstance` (`self.HandMesh`)) State)
  (`self.Multifist` State))

(event `Multifist`
  (params (State :type Boolean))
  ;[0.191 0.5347 1] Update Hands State
  ;;[1 0.7169 0.121] Client update hands' state on server
  (message `/Game/MyContent/Blueprints/Interfaces/AnimationInterface.SendBool1` (`SkeletalMeshComponent.GetAnimInstance` (`self.HandMesh`)) State))

(event `ActivateTeleport`
  (params (isTeleportActive :type Boolean))
  (set `self.isTeleportActive` isTeleportActive))

(event `self.ReceiveTick`
  (params (DeltaSeconds :type "Float (single-precision)"))
  (bind _location (.location (`SceneComponent.K2_GetComponentToWorld` (`self.TeleportPoint`))))
  (`|ExecutionSequence`
    (:`then_0`
      ;[0.1603 1 0.3702] Check Teleport Ability with Visual Teleportation Line
      (if (`self.isTeleportActive`)
        (bind (_outhit _returnvalue) (`KismetSystemLibrary.LineTraceSingle` _location (+ _location (* (`KismetMathLibrary.GetForwardVector` (.rotation (`SceneComponent.K2_GetComponentToWorld` (`self.TeleportPoint`)))) 1500.0)) "TraceTypeQuery1"))
        (if _returnvalue
          (bind (_bblockinghit _binitialoverlap _time _distance _location_2) (`GameplayStatics.BreakHitResult` _outhit))
          (bind _returnvalue_2 (== _location_2 (`NavigationSystemV1.K2_ProjectPointToNavigation` (`NavigationSystemV1.GetNavigationSystem`) _location_2 null null (0.0 0.0 0.0)) :`ErrorTolerance` 15.0))
          (`KismetSystemLibrary.LineTraceSingle` :`Start` _location :`End` _location_2 :`TraceChannel` "TraceTypeQuery1" :`DrawDebugType` "ForOneFrame" :`TraceColor` (`KismetMathLibrary.SelectColor` (struct :`B` 1.0 :`A` 1.0) (struct :`R` 1.0 :`A` 1.0) _returnvalue_2))
          (set `self.CanTeleport?` _returnvalue_2)
          (else
            (set `self.CanTeleport?` false)))))
    (:`then_1`
      ;[0.2598 0.5153 1] Update Client's Hands Locations on Server
      (`/Engine/EditorBlueprintResources/ActorMacros.Switch Has Authority`
        (:`Remote`
          (`self.ServerTick` (`SceneComponent.K2_GetComponentToWorld` (`self.HandPoint`))))))))

(event `ServerTick`
  (params (NewTransform :type "Transform Structure (by ref)"))
  ;[0.2598 0.5153 1] Update Client's Hands Locations on Server
  (`SceneComponent.K2_SetWorldTransform` (`self.HandPoint`) NewTransform false false))

(fn `RecieveTeleportPoint`
  (returns (Point :type "Vector Structure"))
  (bind _location (.location (`SceneComponent.K2_GetComponentToWorld` (`self.TeleportPoint`))))
  (bind _outhit (`KismetSystemLibrary.LineTraceSingle` _location (+ _location (* (`KismetMathLibrary.GetForwardVector` (.rotation (`SceneComponent.K2_GetComponentToWorld` (`self.TeleportPoint`)))) 1500.0)) "TraceTypeQuery1"))
  (return (`.Location` (`GameplayStatics.BreakHitResult` _outhit))))

(fn `UserConstructionScript`)